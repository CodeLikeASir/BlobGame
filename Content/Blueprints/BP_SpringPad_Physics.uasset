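; Physics-driven spring pad that launches player characters when its mesh springs upward.
; A sphere trigger tracks overlapping BP_PlayerCharacter actors.
; Tick watches the mesh's vertical velocity: a fast rise applies a one-shot acceleration force to each capsule along the Plane's up vector, scaled by LaunchForceScalar.
; A fast downward move re-arms the launch latch, and vertical speed prints for debugging while the mesh moves.
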(event `self.ReceiveTick`
  (params (DeltaSeconds :type "Float (single-precision)"))
  (bind (_returnvalue_x _returnvalue_y _returnvalue_z) (`KismetMathLibrary.BreakVector` (`SceneComponent.GetComponentVelocity` (`self.StaticMesh`))))
  (`|ExecutionSequence`
    (:`then_0`
      (if (< _returnvalue_z -100.0)
        (set `self.HasLaunched` false)))
    (:`then_1`
      (if (and (> _returnvalue_z 100.0) (not (`self.HasLaunched`)))
        (set `self.HasLaunched` true)
        (for _array_element (`self.OverlappedActors`)
          (`PrimitiveComponent.AddForce` (`Blob_PlayerCharacter.CapsuleComponent` _array_element) (* (`SceneComponent.GetUpVector` (`self.Plane`)) (* (`self.LaunchForceScalar`) 1000000.0)) "None" true))))
    (:`then_2`
      (if (> (`KismetMathLibrary.Abs` _returnvalue_z) 10.0)
        (`KismetSystemLibrary.PrintText` (`|FormatText` "Speed: {spd}" _returnvalue_z))))))

(event `self.Sphere.OnComponentBeginOverlap`
  (params (OverlappedComponent :type "PrimitiveComponent Object Reference") (OtherActor :type "Actor Object Reference") (OtherComp :type "PrimitiveComponent Object Reference") (OtherBodyIndex :type Integer) (bFromSweep :type Boolean) (SweepResult :type "HitResult Structure (by ref)"))
  (bind _asbp_player_character (cast `/Game/Blueprints/Player/BP_PlayerCharacter` OtherActor))
  (`KismetArrayLibrary.Array_AddUnique` (`self.OverlappedActors`) _asbp_player_character))

(event `self.Sphere.OnComponentEndOverlap`
  (params (OverlappedComponent :type "PrimitiveComponent Object Reference") (OtherActor :type "Actor Object Reference") (OtherComp :type "PrimitiveComponent Object Reference") (OtherBodyIndex :type Integer))
  (bind _asbp_player_character (cast `/Game/Blueprints/Player/BP_PlayerCharacter` OtherActor))
  (`KismetArrayLibrary.Array_RemoveItem` (`self.OverlappedActors`) _asbp_player_character))

(fn `UserConstructionScript`)