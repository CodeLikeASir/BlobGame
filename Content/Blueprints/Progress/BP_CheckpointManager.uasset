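; BP_CheckpointManager records checkpoint progress in the savegame and selects a current checkpoint on load.
; On BeginPlay it caches BP_GameInstance, which OnCheckpointReachedBP uses to store the reached index and current time, then save.
; LoadGame scans all BP_Checkpoint actors and sets the current checkpoint to the one with the highest index above the current index, without reading the savegame.
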(event `self.ReceiveBeginPlay`
  (bind _asbp_game_instance (cast `/Game/Blueprints/Core/BP_GameInstance` (`GameplayStatics.GetGameInstance`)))
  (set `self.GameInstance` _asbp_game_instance))

(event `self.OnCheckpointReachedBP`
  (params (CheckpointIndex :type Integer))
  (bind _returnvalue (`Blob_GameInstance.GetSavegame` (`self.GameInstance`)))
  (set `Blob_Savegame.LastCheckpointIndex` CheckpointIndex _returnvalue)
  (set `Blob_Savegame.LastCheckpointTime` (`Blob_GameInstance.GetCurrentTime` (`self.GameInstance`)) _returnvalue)
  (`Blob_GameInstance.SaveSavegame` (`self.GameInstance`)))

(event `LoadGame`
  (bind _outactors (`GameplayStatics.GetAllActorsOfClass` "/Game/Blueprints/Progress/BP_Checkpoint.BP_Checkpoint_C"))
  (for _array_element _outactors
    (if (> (`Blob_Checkpoint.CheckpointIndex` _array_element) (`self.CurrentCheckpointIndex`))
      (set `self.CurrentCheckpoint` (`|ConvertAsset` _array_element))
      (set `self.CurrentCheckpointIndex` (`Blob_Checkpoint.CheckpointIndex` _array_element)))))

(fn `UserConstructionScript`)