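; Player character Blueprint for a blob with eyes, handling visual and audio feedback for jump, hit reaction and downforce, plus collectable counting.
; A dynamic body material shows charge progress every tick, flashes red on hits and turns dark and opaque during downforce, which also swaps to a squished mesh and hides the eyes.
; Jump release plays sound and a scale-reset timeline; overlapping non-movable actors stops downforce.
; BeginPlay registers the character with the checkpoint manager.
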(event `self.ReceiveBeginPlay`
  (bind _returnvalue (`PrimitiveComponent.CreateDynamicMaterialInstance` (`self.BlobMesh`) 0 "/Game/Materials/Mat_Body.Mat_Body" "None"))
  (set `self.Material` _returnvalue)
  (bind _asbp_player_controller (cast `/Game/Blueprints/Core/BP_PlayerController` (`GameplayStatics.GetPlayerController` 0)))
  (set `self.PlayerController` _asbp_player_controller)
  (bind _returnvalue_2 (`GameplayStatics.GetActorOfClass` "/Game/Blueprints/Progress/BP_CheckpointManager.BP_CheckpointManager_C"))
  (set `Blob_CheckpointManager.PlayerCharacter` self _returnvalue_2)
  (bind _returnvalue_3 (`MaterialInstanceDynamic.K2_GetScalarParameterValue` (`self.Material`) (`self.MatParam_Opacity`)))
  (set `self.DefaultOpacity` _returnvalue_3))

(event `self.ReceiveTick`
  (params (DeltaSeconds :type "Float (single-precision)"))
  (`MaterialInstanceDynamic.SetScalarParameterValue` (`self.Material`) (`self.MatParam_ChargeProgress`) (`self.ChargeProgress`)))

(event `self.ReleaseJumpBP`
  (bind _sfx_jump (`self.SFX_Jump`))
  (if (`AudioComponent.IsPlaying` _sfx_jump)
    (bind (_direction _meshscalelerpalpha) (`Timeline|ResetScale` :!via `PlayFromStart` :!label _label)
      (:`Update`
        (`SceneComponent.SetRelativeScale3D` (`self.BlobMesh`) (`KismetMathLibrary.VLerp` (`self.SquishScale`) (`self.BaseScale`) _meshscalelerpalpha))))
    (else
      (`AudioComponent.Play` _sfx_jump 0.0)
      (goto _label :!via `PlayFromStart`))))

(event `self.BeginHitReactionBP`
  (params (UnlockTime :type "Float (single-precision)"))
  ; Hit Reaction
  (`MaterialInstanceDynamic.SetScalarParameterValue` (`self.Material`) (`self.MatParam_CustomBlend`) 1.0)
  (`MaterialInstanceDynamic.SetVectorParameterValue` (`self.Material`) (`self.MatParam_CustomColor`) (struct :`R` 1.0 :`A` 1.0)))

(event `self.EndHitReactionBP`
  ; Hit Reaction
  (`MaterialInstanceDynamic.SetScalarParameterValue` (`self.Material`) (`self.MatParam_CustomBlend`) 0.0))

(event `self.StartDownforceBP`
  ; Downforce Visuals
  (`StaticMeshComponent.SetStaticMesh` (`self.BlobMesh`) "/Game/Meshes/PlayerBody_Squished.PlayerBody_Squished")
  (`SceneComponent.SetVisibility` (`self.EyeRight`) false false)
  (`SceneComponent.SetVisibility` (`self.EyeLeft`) false false)
  (`MaterialInstanceDynamic.SetScalarParameterValue` (`self.Material`) (`self.MatParam_CustomBlend`) 1.0)
  (`MaterialInstanceDynamic.SetVectorParameterValue` (`self.Material`) (`self.MatParam_CustomColor`) (struct :`R` 0.010417 :`G` 0.010417 :`B` 0.010417 :`A` 1.0))
  (`MaterialInstanceDynamic.SetScalarParameterValue` (`self.Material`) (`self.MatParam_Opacity`) 1.0))

(event `self.StopDownforceBP`
  ; Downforce Visuals
  (`StaticMeshComponent.SetStaticMesh` (`self.BlobMesh`) "/Game/Meshes/PlayerBody.PlayerBody")
  (`SceneComponent.SetVisibility` (`self.EyeRight`) true false)
  (`SceneComponent.SetVisibility` (`self.EyeLeft`) true false)
  (`MaterialInstanceDynamic.SetScalarParameterValue` (`self.Material`) (`self.MatParam_CustomBlend`) 0.0)
  (`MaterialInstanceDynamic.SetScalarParameterValue` (`self.Material`) (`self.MatParam_Opacity`) (`self.DefaultOpacity`)))

(event `self.ReceiveActorBeginOverlap`
  (params (OtherActor :type "Actor Object Reference"))
  (`/Engine/EditorBlueprintResources/StandardMacros.IsValid` OtherActor
    (:`Is Valid`
      (if (`|EnumInequality` (`SceneComponent.Mobility` (`Actor.RootComponent` OtherActor)) "Movable")
        (`self.StopDownforce`)))))

(event `self.PickupCollectable`
  (bind _result (`/Engine/EditorBlueprintResources/StandardMacros.IncrementInt` (`self.CurrentCollectables`))
    (:`  `
      (`/Game/Blueprints/Core/BP_PlayerController.ShowMessage` (`self.PlayerController`) (`|FormatText` "Collected {current} / {total} collectables" _result (`self.TotalCollectables`)) 2.0))))

(fn `UserConstructionScript`)