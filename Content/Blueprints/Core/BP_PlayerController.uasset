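; Player controller for a checkpoint-based, timed game that owns the menu, HUD and win screen flow.
; On begin play it registers with the checkpoint manager and creates widgets, later seeding the HUD with saved checkpoint times.
; Respawning teleports the pawn above its checkpoint and resets the camera arm, except in hardcore mode.
; Pausing uses zero global time dilation, and P jumps to the next checkpoint.
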(event `self.ReceiveBeginPlay`
  (set `self.MainMenuOpen` true)
  (bind _asbp_game_instance (cast `/Game/Blueprints/BP_GameInstance` (`GameplayStatics.GetGameInstance`)))
  (set `self.GameInstance` _asbp_game_instance)
  (bind _returnvalue (`GameplayStatics.GetActorOfClass` "/Game/Blueprints/BP_CheckpointManager.BP_CheckpointManager_C"))
  (bind _output_get (set `self.CheckpointManager` _returnvalue))
  (set `Blob_CheckpointManager.PlayerController` self _output_get)
  (bind _returnvalue_2 (`|CreateWidget` "/Game/Blueprints/UI/WBP_MainMenu.WBP_MainMenu_C" self))
  (`UserWidget.AddToViewport` _returnvalue_2 0)
  (bind _returnvalue_3 (`|CreateWidget` "/Game/Blueprints/UI/WBP_PlayerHUD.WBP_PlayerHUD_C" self))
  (bind _output_get_2 (set `self.PlayerHUD` _returnvalue_3))
  (`UserWidget.AddToViewport` _output_get_2 0))

(event `self.RespawnBP`
  (`/Game/Blueprints/UI/WBP_PlayerHUD.ClearNotification` (`self.PlayerHUD`) :!label _label)
  (bind _returnvalue (`Blob_GameUserSettings.GetCustomSettings`))
  (if (`Blob_GameUserSettings.bIsHardcoreMode` _returnvalue)
    (`/Game/Blueprints/UI/WBP_PlayerHUD.ShowMessage` (`self.PlayerHUD`) "No checkpoints in hardcore." 2.0)
    (else
      (`self.ResetToCheckpoint`))))

(event `ForceRespawn`
  (params (Delay :type "Float (double-precision)"))
  (`KismetSystemLibrary.Delay` Delay)
  (goto _label))

(event `self.OpenPauseMenu`
  (if (not (`self.MainMenuOpen`))
    (bind _returnvalue (`|CreateWidget` "/Game/Blueprints/UI/WBP_MainMenu.WBP_MainMenu_C" self))
    (`UserWidget.AddToViewport` _returnvalue 0)
    (`GameplayStatics.SetGlobalTimeDilation` 0.0)
    (`WidgetBlueprintLibrary.SetInputMode_UIOnlyEx` self _returnvalue)
    (set `self.bShowMouseCursor` true)
    (set `self.MainMenuOpen` true)))

(event `self.OnCheckpointReachedBP`
  (params (Index :type Integer))
  (`/Game/Blueprints/UI/WBP_PlayerHUD.OnCheckpointReached` (`self.PlayerHUD`) Index)
  (`/Game/Blueprints/UI/WBP_PlayerHUD.ShowMessage` (`self.PlayerHUD`) (`self.GetEnteredStageMessage` Index) 1.5))

(event `StartGame`
  (bind _returnvalue (`Blob_GameInstance.GetSavegame` (`self.GameInstance`)))
  (`/Game/Blueprints/UI/WBP_PlayerHUD.InitAndStart` (`self.PlayerHUD`) (`Blob_Savegame.CheckpointTimes` _returnvalue)))

(event `Key|P`
  (params (Key :type "Key Structure"))
  (:`Pressed`
    (`self.JumpToNextCheckpoint`)))

(event `ResetTimes`
  (`/Game/Blueprints/UI/WBP_PlayerHUD.ResetTimes` (`self.PlayerHUD`)))

(event `self.OnGameEndBP`
  (bind _returnvalue (`|CreateWidget` "/Game/Blueprints/UI/WBP_WinScreen.WBP_WinScreen_C" self))
  (`UserWidget.AddToViewport` _returnvalue 0))

(event `self.ShowResetNotification`
  (bind _returnvalue (`Blob_GameUserSettings.GetCustomSettings`))
  (if (not (`Blob_GameUserSettings.bIsHardcoreMode` _returnvalue))
    (`/Game/Blueprints/UI/WBP_PlayerHUD.ShowResetNotification` (`self.PlayerHUD`))))

(event `self.ClearNotifications`
  (`/Game/Blueprints/UI/WBP_PlayerHUD.ClearNotification` (`self.PlayerHUD`)))

(fn `ShowMessage`
  (params (Message :type Text) (Time :type "Float (double-precision)"))
  (`/Game/Blueprints/UI/WBP_PlayerHUD.ShowMessage` (`self.PlayerHUD`) Message Time))

(fn `UserConstructionScript`)