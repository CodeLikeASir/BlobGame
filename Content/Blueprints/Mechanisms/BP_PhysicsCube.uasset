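; BP_PhysicsCube is a mechanism actor that registers itself as a resettable object with the nearest BP_ObjectResetter in the level.
; On BeginPlay it scans every BP_ObjectResetter, tracks the closest by distance, then calls RegisterResettable on it.
; The link is resolved by proximity at runtime, and the reset behavior itself lives outside this graph.
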(event `self.ReceiveBeginPlay`
  (bind _outactors (`GameplayStatics.GetAllActorsOfClass` "/Game/Blueprints/Mechanisms/BP_ObjectResetter.BP_ObjectResetter_C"))
  (for _array_element _outactors
    (bind _returnvalue (`KismetMathLibrary.Vector_Distance` (`self.K2_GetActorLocation` _array_element) (`self.K2_GetActorLocation`)))
    (if (< _returnvalue (`self.NearestResetterDist`))
      (set `self.NearestResetterDist` _returnvalue)
      (set `self.NearestResetter` _array_element)))
  (`Blob_ObjectResetter.RegisterResettable` (`self.NearestResetter`) self))

(fn `UserConstructionScript`)