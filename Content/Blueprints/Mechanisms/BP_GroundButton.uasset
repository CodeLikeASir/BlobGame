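; A ground button mechanism that switches on and off according to the height offset of its button component.
; Tick compares GetZOffset against separate on and off thresholds, allowing hysteresis, and calls OnToggled when the state flips.
; OnToggled swaps the button material and calls OnToggleOn or OnToggleOff for the response.
; The GetZOffset graph shows only an unconnected Button-minus-Ground Z subtraction.
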(event `self.ReceiveTick`
  (params (DeltaSeconds :type "Float (single-precision)"))
  (bind _offset (`self.GetZOffset`))
  (if (`self.IsOn`)
    (if (> _offset (`self.OffThreshold`))
      (set `self.IsOn` false)
      (`self.OnToggled` :!label _label))
    (elif (< _offset (`self.OnThreshold`))
      (set `self.IsOn` true)
      (goto _label))))

(event `OnToggled`
  (bind _button (`self.Button`))
  (if (`self.IsOn`)
    (`PrimitiveComponent.SetMaterial` _button 0 (`self.OnMaterial`))
    (else
      (`PrimitiveComponent.SetMaterial` _button 0 (`self.OffMaterial`))))
  (if (`self.IsOn`)
    (`self.OnToggleOn`)
    (else
      (`self.OnToggleOff`))))

(fn `UserConstructionScript`)