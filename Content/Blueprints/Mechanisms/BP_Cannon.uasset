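; Toggle-driven cannon mechanism that aims at a Target component and fires one projectile per switch-on, re-arming on switch-off.
; ForceUpdate or OnComponentMoved yaws the Turret and pitches the Barrel toward Target, then places ProjectileSpawn along the barrel's right vector, which serves as its forward axis.
; Firing spawns ProjectileClass there and sets its movement velocity along the barrel-to-spawn direction, scaled by InitialVelocity.
; Debug shapes and text show the muzzle and shot.
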(event `ForceUpdate`
  (bind _barrel (`self.Barrel`))
  (bind _returnvalue (`SceneComponent.K2_GetComponentLocation` (`self.ProjectileSpawn`)))
  (bind (_returnvalue_roll _returnvalue_pitch _returnvalue_yaw) (`KismetMathLibrary.BreakRotator` (`KismetMathLibrary.FindLookAtRotation` (`SceneComponent.K2_GetComponentLocation` (`self.Turret`)) (`SceneComponent.K2_GetComponentLocation` (`self.Target`)))))
  (bind (_returnvalue_roll_2 _returnvalue_pitch_2) (`KismetMathLibrary.BreakRotator` (`KismetMathLibrary.FindLookAtRotation` (`SceneComponent.K2_GetComponentLocation` (`self.Barrel`)) (`SceneComponent.K2_GetComponentLocation` (`self.Target`)))))
  (bind _returnvalue_2 (* (`SceneComponent.GetRightVector` _barrel) (`self.SpawnOffset`)))
  (bind _returnvalue_3 (+ (`SceneComponent.K2_GetComponentLocation` _barrel) _returnvalue_2))
  (`SceneComponent.K2_SetWorldRotation` (`self.Turret`) (`KismetMathLibrary.MakeRotator` 0.0 0.0 (+ _returnvalue_yaw -90.0)) false false :!label _label)
  (`SceneComponent.K2_SetRelativeRotation` (`self.Barrel`) (`KismetMathLibrary.MakeRotator` (* _returnvalue_pitch_2 -1.0)) false false)
  (`KismetSystemLibrary.DrawDebugSphere` _returnvalue_3 5.0 12 (struct :`G` 0.077789 :`B` 1.0 :`A` 1.0) 5.0 2.0)
  (`SceneComponent.K2_SetWorldLocation` (`self.ProjectileSpawn`) _returnvalue_3 false false)
  (`SceneComponent.K2_SetWorldRotation` (`self.ProjectileSpawn`) (`KismetMathLibrary.FindLookAtRotation` _returnvalue (+ _returnvalue _returnvalue_2)) false false))

(event `self.OnComponentMoved`
  (goto _label))

(event `self.OnToggleOff`
  (set `self.CanFire` true))

(event `self.OnToggleOn`
  (bind _returnvalue (`SceneComponent.K2_GetComponentLocation` (`self.ProjectileSpawn`)))
  (if (`self.CanFire`)
    (`KismetSystemLibrary.PrintText` "BOOM")
    (set `self.CanFire` false)
    (bind _returnvalue_2 (`self.GetCannonForward`))
    (bind _returnvalue_3 (`|SpawnActorFromClass` (`self.ProjectileClass`) (`KismetMathLibrary.MakeTransform` (`SceneComponent.K2_GetComponentLocation` (`self.ProjectileSpawn`)) (struct) (0.65 0.65 0.65)) "AlwaysSpawn" "MultiplyWithRoot" null null))
    (bind _returnvalue_4 (* _returnvalue_2 (`self.InitialVelocity`)))
    (set `MovementComponent.Velocity` _returnvalue_4 (`self.GetComponentByClass` _returnvalue_3 "/Script/Engine.ProjectileMovementComponent"))
    (`KismetSystemLibrary.DrawDebugLine` _returnvalue (+ _returnvalue _returnvalue_4) (struct :`R` 1.0 :`B` 0.434923 :`A` 1.0) 3.0 2.0)))

(fn `GetCannonForward`
  (returns (ReturnValue :type "Vector Structure"))
  (return (`KismetMathLibrary.Normal` (- (`SceneComponent.K2_GetComponentLocation` (`self.ProjectileSpawn`)) (`SceneComponent.K2_GetComponentLocation` (`self.Barrel`))))))

(fn `UserConstructionScript`)