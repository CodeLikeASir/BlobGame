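; BP_RotatingBlock is a mechanism actor that rotates in repeated steps with a pause between each.
; BeginPlay starts the Rotating timeline, which lerps the actor's rotation from CurrentStart to CurrentEnd along the shortest path.
; When it finishes, it waits PauseLength, combines the current rotation with RotationDir for the next target, and replays.
; OnToggleon and OnToggleOff resume and stop the timeline.
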(event `self.ReceiveBeginPlay`
  (bind (_direction _rotating) (`Timeline|Rotating` :!via `PlayFromStart` :!label _label)
    (:`Update`
      (`self.K2_SetActorRotation` (`KismetMathLibrary.RLerp` (`self.CurrentStart`) (`self.CurrentEnd`) _rotating true)))
    (:`Finished`
      (`KismetSystemLibrary.Delay` (`self.PauseLength`))
      (bind _output_get (set `self.CurrentStart` (`self.K2_GetActorRotation`)))
      (set `self.CurrentEnd` (`KismetMathLibrary.ComposeRotators` _output_get (`self.RotationDir`)))
      (goto _label :!via `PlayFromStart`))))

(event `self.OnToggleOn`
  (goto _label))

(event `self.OnToggleOff`
  (goto _label :!via `Stop`))

(fn `UserConstructionScript`)