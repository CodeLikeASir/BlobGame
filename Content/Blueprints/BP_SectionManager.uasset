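; Section manager actor that groups a part of the level through actor attachment and tracks that section's checkpoint.
; On BeginPlay it stores the BP_Checkpoint attached to it and hides the section if its ProgressIndex is above zero.
; ToggleVisibility shows or hides directly attached actors, without recursing or changing collision.
; GetCheckpointLocation exposes the stored checkpoint's world position.
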(event `self.ReceiveBeginPlay`
  (bind _outactors (`GameplayStatics.GetAllActorsOfClass` "/Game/Blueprints/BP_Checkpoint.BP_Checkpoint_C"))
  (for _array_element _outactors
    (if (== (`self.GetAttachParentActor` _array_element) self)
      (set `self.Checkpoint` _array_element)))
  (if (> (`self.ProgressIndex`) 0)
    (`self.ToggleVisibility` false)))

(event `ToggleVisibility`
  (params (IsVisible :type Boolean))
  (for _array_element (`self.GetAttachedActors` true)
    (`self.SetActorHiddenInGame` _array_element (not IsVisible))))

(fn `GetCheckpointLocation`
  (returns (Location :type "Vector Structure"))
  (return (`self.K2_GetActorLocation` (`self.Checkpoint`))))

(fn `UserConstructionScript`)