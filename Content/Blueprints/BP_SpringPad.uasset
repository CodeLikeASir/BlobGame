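; BP_SpringPad is a spring pad that launches an overlapping Character along the pad's up vector.
; An overlap plays a timeline that lerps the mesh between its base location and an offset along negative mesh up, driven by a spring-like curve.
; The launch fires when the timeline finishes, scaled by SpringStrength and overriding existing velocity.
; An InProgress flag blocks retriggering during the animation.
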(event `self.ReceiveBeginPlay`
  (bind _staticmesh (`self.StaticMesh`))
  (bind _relativelocation (`SceneComponent.RelativeLocation` _staticmesh))
  (set `self.BaseLocation` _relativelocation)
  (set `self.AnimTarget` (- _relativelocation (* (`SceneComponent.GetUpVector` _staticmesh) (`self.AnimStrength`)))))

(event `self.ReceiveActorBeginOverlap`
  (params (OtherActor :type "Actor Object Reference"))
  (if (not (`self.InProgress`))
    (bind (_direction _springpseudoanim) (`Timeline|Timeline` :!via `PlayFromStart`)
      (:`Update`
        (set `self.InProgress` true)
        (`SceneComponent.K2_SetRelativeLocation` (`self.StaticMesh`) (`KismetMathLibrary.VLerp` (`self.BaseLocation`) (`self.AnimTarget`) _springpseudoanim) false false))
      (:`Finished`
        (bind _ascharacter (cast `Character` OtherActor))
        (`Character.LaunchCharacter` _ascharacter (* (`self.GetActorUpVector`) (* (`self.SpringStrength`) 1000.0)) true true)
        (set `self.InProgress` false)))))

(fn `UserConstructionScript`)