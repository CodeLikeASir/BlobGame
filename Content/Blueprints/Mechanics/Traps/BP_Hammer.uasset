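; BP_Hammer is a swinging hammer trap that launches the player character it hits.
; A timeline with configurable curve, duration, offset and speed drives the mesh pitch and triggers a whoosh sound.
; Each update records the SpeedHelper component's position and stores GetMoveVec's result as Velocity.
; Overlap applies that velocity to the player's capsule as physics linear velocity, then blocks relaunching for a short cooldown.
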(event `self.ReceiveBeginPlay`
  (`TimelineComponent.SetTimelineLength` (`self.SpeedTimeline`) (`self.CurveDuration`))
  (`TimelineComponent.SetNewTime` (`self.SpeedTimeline`) (`self.TimeOffset`))
  (`TimelineComponent.SetPlayRate` (`self.SpeedTimeline`) (`self.SpeedMultiplier`))
  (`TimelineComponent.SetFloatCurve` (`self.SpeedTimeline`) (`self.FloatCurve`) "Rotation")
  (bind (_direction _rotation) (`Timeline|SpeedTimeline`)
    (:`Update`
      (set `self.LastPos` (`SceneComponent.K2_GetComponentLocation` (`self.SpeedHelper`)))
      (`SceneComponent.K2_SetRelativeRotation` (`self.StaticMesh`) (`KismetMathLibrary.MakeRotator` 0.0 (* _rotation (`self.MaxAngle`))) false false)
      (set `self.Velocity` (`self.GetMoveVec`)))
    (:`SoundFX`
      (`AudioComponent.Play` (`self.Whoosh_Cue`) 0.0))))

(event `self.ReceiveActorBeginOverlap`
  (params (OtherActor :type "Actor Object Reference"))
  (if (and (> (`self.ForceMultiplier`) 0.0) (`self.CanLaunch`))
    (bind _asbp_player_character (cast `/Game/Blueprints/Core/BP_PlayerCharacter` OtherActor))
    (`PrimitiveComponent.SetPhysicsLinearVelocity` (`Blob_PlayerCharacter.CapsuleComponent` _asbp_player_character) (`self.Velocity`) false "None")
    (set `self.CanLaunch` false)
    (`KismetSystemLibrary.K2_SetTimerDelegate` (delegate `EnableLaunch`) 2.0)))

(event `EnableLaunch`
  (set `self.CanLaunch` true))

(fn `UserConstructionScript`)