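; BP_SpikeBlock is a trap actor that rotates in repeated steps with a pause between each.
; The Rotating timeline lerps the actor along the shortest path from CurrentStart to CurrentEnd, which UpdateStartEnd derives by combining the current rotation with RotationDir.
; On finish it waits PauseLength, recomputes both rotations and replays.
; TimeOffset staggers the first cycle, and OnToggleon and OnToggleOff play or stop the timeline.
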(event `self.ReceiveBeginPlay`
  (`self.UpdateStartEnd`)
  (`TimelineComponent.SetNewTime` (`self.Rotating`) (`self.TimeOffset`))
  (bind (_direction _rotating) (`Timeline|Rotating` :!label _label)
    (:`Update`
      (`self.K2_SetActorRotation` (`KismetMathLibrary.RLerp` (`self.CurrentStart`) (`self.CurrentEnd`) _rotating true)))
    (:`Finished`
      (`KismetSystemLibrary.Delay` (`self.PauseLength`))
      (`self.UpdateStartEnd`)
      (goto _label :!via `PlayFromStart`))))

(event `self.OnToggleOn`
  (goto _label))

(event `self.OnToggleOff`
  (goto _label :!via `Stop`))

(fn `UserConstructionScript`)