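; BP_GroundLever is an interactable lever that acts as an on/off switch.
; BeginPlay sets the handle to a tilted starting rotation, and Tick derives IsOn from whether its relative roll is above zero.
; Only when that state flips, it calls OnToggleOn or OnToggleOff and swaps the handle top's material to green or red.
; The file only reads the handle's rotation after setup, with no logic here that moves it.
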(event `self.ReceiveBeginPlay`
  (`SceneComponent.K2_SetRelativeRotation` (`self.LeverHandle`) (struct :`Roll` -30.0) false false))

(event `self.ReceiveTick`
  (params (DeltaSeconds :type "Float (single-precision)"))
  (bind _leverhandletop (`self.LeverHandleTop`))
  (bind _relativerotation_roll (`KismetMathLibrary.BreakRotator` (`SceneComponent.RelativeRotation` (`self.LeverHandle`))))
  (bind _returnvalue (> _relativerotation_roll 0.0))
  (if (!= _returnvalue (`self.IsOn`))
    (bind _output_get (set `self.IsOn` _returnvalue))
    (if _output_get
      (`self.OnToggleOn`)
      (`PrimitiveComponent.SetMaterial` _leverhandletop 0 "/Game/Materials/Mat_Green.Mat_Green")
      (else
        (`self.OnToggleOff`)
        (`PrimitiveComponent.SetMaterial` _leverhandletop 0 "/Game/Materials/Mat_Red.Mat_Red")))))

(fn `UserConstructionScript`)