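; Player camera actor that lengthens its spring arm as player pawn 0 gets farther from it.
; It caches the pawn on BeginPlay and checks the distance every Tick.
; Beyond a threshold, the excess distance maps to a clamped range of arm lengths, eased in with FInterpTo.
; Inside the threshold the arm length is left unchanged, with no return to a base value.
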(event `self.ReceiveBeginPlay`
  (set `self.Player` (`GameplayStatics.GetPlayerPawn` 0)))

(event `self.ReceiveTick`
  (params (DeltaSeconds :type "Float (single-precision)"))
  (bind _returnvalue (`KismetMathLibrary.Vector_Distance` (`self.K2_GetActorLocation`) (`self.K2_GetActorLocation` (`self.Player`))))
  (if (> _returnvalue 800.0)
    (set `SpringArmComponent.TargetArmLength` (`KismetMathLibrary.FInterpTo` (`SpringArmComponent.TargetArmLength` (`self.CameraArmComponent`)) (+ (* (`KismetMathLibrary.FClamp` (/ (- _returnvalue 800.0) 1000.0)) 1500.0) 1700.0) DeltaSeconds 2.0) (`self.CameraArmComponent`))))

(fn `UserConstructionScript`)