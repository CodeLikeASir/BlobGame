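; Player controller that relays respawn requests and a checkpoint shortcut to the game mode.
; On begin play it caches the BP_GameMode reference.
; RespawnBP asks the game mode to respawn the player character, then resets the custom player camera, and the 2 key unlocks the next checkpoint.
; Main menu widget creation is present but disconnected, so it never runs.
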(event `self.ReceiveBeginPlay`
  (bind _asbp_game_mode (cast `/Game/Blueprints/BP_GameMode` (`GameplayStatics.GetGameMode`)))
  (set `self.GameMode` _asbp_game_mode))

(event `self.RespawnBP`
  (`/Game/Blueprints/BP_GameMode.RespawnPlayer` (`self.GameMode`) (`self.PlayerCharacter`))
  (`Blob_PlayerCamera.ResetCamera` (`self.CustomPlayerCamera`)))

(event `Key|Two`
  (params (Key :type "Key Structure"))
  (:`Pressed`
    (`/Game/Blueprints/BP_GameMode.UnlockedNextCheckpoint` (`self.GameMode`))))

(fn `UserConstructionScript`)