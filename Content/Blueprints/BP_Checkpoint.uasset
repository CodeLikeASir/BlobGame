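; BP_Checkpoint is a checkpoint actor that plays a Niagara burst effect at its location when its OnCheckpointReached event fires.
; On BeginPlay it casts and caches the BP_GameMode, though no live logic uses that reference.
; A sound playback gated on the game mode's running state and a level-number parse from the level name are left disconnected.
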(event `self.ReceiveBeginPlay`
  (bind _asbp_game_mode (cast `/Game/Blueprints/BP_GameMode` (`GameplayStatics.GetGameMode`)))
  (set `self.GameMode` _asbp_game_mode))

(event `self.OnCheckpointReached`
  (`NiagaraFunctionLibrary.SpawnSystemAtLocation` "/Game/VFX/NS_CheckpointBurst.NS_CheckpointBurst" (`self.K2_GetActorLocation`)))

(fn `UserConstructionScript`)