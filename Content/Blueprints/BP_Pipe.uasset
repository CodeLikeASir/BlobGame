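; Two-way travel pipe that carries the player character along a spline between entrances EnterA and EnterB.
; The construction script builds the tube from collidable spline mesh segments between consecutive spline points.
; Overlapping an entrance claims one player at a time, hides them by zero scale, and plays a shared Timeline forward or in reverse.
; The Timeline moves them along the spline at constant velocity, then restores unit scale and releases them.
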(event `self.ReceiveBeginPlay`
  (add `PrimitiveComponent.OnComponentBeginOverlap` (`self.EnterA`) (delegate `OverlapA`))
  (add `PrimitiveComponent.OnComponentBeginOverlap` (`self.EnterB`) (delegate `OverlapB`)))

(event `OverlapA`
  (params (OverlappedComponent :type "PrimitiveComponent Object Reference") (OtherActor :type "Actor Object Reference") (OtherComp :type "PrimitiveComponent Object Reference") (OtherBodyIndex :type Integer) (bFromSweep :type Boolean) (SweepResult :type "HitResult Structure (by ref)"))
  (`self.CheckMovedActor` OtherActor)
  (bind (_direction _progress) (`Timeline|Timeline` :!via `PlayFromStart` :!label _label)
    (:`Update`
      (`self.K2_SetActorLocation` (`self.MovedActor`) (`SplineComponent.GetLocationAtTime` (`self.Spline`) _progress "World" true) false false))
    (:`Finished`
      (`self.SetActorScale3D` (`self.MovedActor`) (1.0 1.0 1.0))
      (set `self.MovedActor` null))))

(event `OverlapB`
  (params (OverlappedComponent :type "PrimitiveComponent Object Reference") (OtherActor :type "Actor Object Reference") (OtherComp :type "PrimitiveComponent Object Reference") (OtherBodyIndex :type Integer) (bFromSweep :type Boolean) (SweepResult :type "HitResult Structure (by ref)"))
  (`self.CheckMovedActor` OtherActor)
  (goto _label :!via `ReverseFromEnd`))

(fn `UserConstructionScript`
  (bind _spline (`self.Spline`))
  (for _index (range (+ (- (`SplineComponent.GetNumberOfSplinePoints` (`self.Spline`)) 2) 1))
    (bind _returnvalue (`AddComponent|NODE_AddSplineMeshComponent-0`))
    (`StaticMeshComponent.SetStaticMesh` _returnvalue (`self.Mesh`))
    (`SplineMeshComponent.SetForwardAxis` _returnvalue (`self.ForwardAxis`) true)
    (`SceneComponent.K2_AttachToComponent` _returnvalue (`self.Spline`) "None" "KeepRelative" "KeepRelative" "KeepRelative" true)
    (bind _returnvalue_2 (+ _index 1))
    (`SplineMeshComponent.SetStartAndEnd` _returnvalue (`SplineComponent.GetLocationAtSplinePoint` _spline _index "Local") (`SplineComponent.GetTangentAtSplinePoint` _spline _returnvalue_2 "Local") (`SplineComponent.GetLocationAtSplinePoint` _spline _returnvalue_2 "Local") (`SplineComponent.GetTangentAtSplinePoint` _spline (+ _returnvalue_2 1) "Local") true)
    (`PrimitiveComponent.SetCollisionEnabled` _returnvalue "QueryAndPhysics")))