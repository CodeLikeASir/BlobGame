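; BP_CheckpointManager records checkpoint progress to the savegame and loads a background level when play begins.
; On BeginPlay it loads the Background level as a level instance, then caches the game mode as BP_GameMode.
; When a checkpoint is reached, it writes the checkpoint index and the game mode's current time into the savegame, then has the game mode save it.
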(event `self.ReceiveBeginPlay`
  (`LevelStreamingDynamic.LoadLevelInstanceBySoftObjectPtr` "/Game/Maps/Background.Background" (0.0 0.0 0.0) (struct) "" null)
  (bind _asbp_game_mode (cast `/Game/Blueprints/BP_GameMode` (`GameplayStatics.GetGameMode`)))
  (set `self.GameMode` _asbp_game_mode))

(event `self.OnCheckpointReachedBP`
  (params (CheckpointIndex :type Integer))
  (bind _savegame (`/Game/Blueprints/BP_GameMode.GetSavegame` (`self.GameMode`)))
  (set `Blob_Savegame.LastCheckpointIndex` CheckpointIndex _savegame)
  (set `Blob_Savegame.LastCheckpointTime` (`/Game/Blueprints/BP_GameMode.CurrentTime` (`self.GameMode`)) _savegame)
  (`/Game/Blueprints/BP_GameMode.SaveSavegame` (`self.GameMode`)))

(fn `UserConstructionScript`)