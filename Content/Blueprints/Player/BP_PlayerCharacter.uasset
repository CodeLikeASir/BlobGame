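; Player character Blueprint for a blob with a charged jump, handling its visual, audio and physical-material setup.
; Each tick feeds ChargeProgress into a dynamic body material and writes player position and highest Z reached to a Material Parameter Collection.
; Releasing a jump plays a sound and a timeline easing the mesh from squished to base scale.
; A separate start/stop timeline drives uniform-scale breathing.
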(event `self.ReceiveBeginPlay`
  (bind _returnvalue (`PrimitiveComponent.CreateDynamicMaterialInstance` (`self.BlobMesh`) 0 "/Game/Meshes/Mat_Body.Mat_Body" "None"))
  (set `self.Material` _returnvalue)
  (`PrimitiveComponent.SetPhysMaterialOverride` (`self.CapsuleComponent`) "/Game/PM_Blob.PM_Blob")
  (bind _asbp_player_controller (cast `/Game/Blueprints/Player/BP_PlayerController` (`GameplayStatics.GetPlayerController` 0)))
  (set `self.PC` _asbp_player_controller))

(event `self.ReceiveTick`
  (params (DeltaSeconds :type "Float (single-precision)"))
  (`MaterialInstanceDynamic.SetScalarParameterValue` (`self.Material`) "ChargeProgress" (`self.ChargeProgress`))
  (`self.UpdatePlayerPos`))

(event `self.ReleaseJumpBP`
  (`AudioComponent.Play` (`self.SFX_Jump`) 0.0)
  (bind (_direction _meshscalelerpalpha) (`Timeline|ResetScale` :!via `PlayFromStart`)
    (:`Update`
      (`SceneComponent.SetRelativeScale3D` (`self.BlobMesh`) (`KismetMathLibrary.VLerp` (`self.SquishScale`) (`self.BaseScale`) _meshscalelerpalpha)))))

(event `StartBreathing`
  (bind (_direction _newtrack_0) (`Timeline|BreathingTL` :!via `PlayFromStart` :!label _label)
    (:`Update`
      (`SceneComponent.SetRelativeScale3D` (`self.BlobMesh`) (* _newtrack_0 (1.0 1.0 1.0))))))

(event `StopBreathing`
  (goto _label :!via `Stop`))

(fn `UpdatePlayerPos`
  (bind _returnvalue (`self.K2_GetActorLocation`))
  (bind _z (.z _returnvalue))
  (`KismetMaterialLibrary.SetVectorParameterValue` (`self.ParamCollection`) "PlayerPosition" (`KismetMathLibrary.Conv_VectorToLinearColor` _returnvalue))
  (if (> _z (`self.HighestZ`))
    (bind _output_get (set `self.HighestZ` _z))
    (`KismetMaterialLibrary.SetScalarParameterValue` (`self.ParamCollection`) "HighestPlayerPosition" _output_get)
    (return)
    (else
      (return))))

(fn `UserConstructionScript`)