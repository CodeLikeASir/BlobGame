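; Player controller Blueprint that owns the HUD and main menu and handles respawn and pause for the player.
; On begin play it caches the game mode and checkpoint manager, then creates the menu and HUD widgets.
; Respawn teleports the pawn above the last checkpoint and resets the camera arm, unless hardcore mode blocks it.
; Pause reopens the main menu with zero time dilation, while start, checkpoint and message events forward to the HUD.
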(event `self.ReceiveBeginPlay`
  (bind _asbp_game_mode (cast `/Game/Blueprints/BP_GameMode` (`GameplayStatics.GetGameMode`)))
  (set `self.GameMode` _asbp_game_mode)
  (bind _returnvalue (`GameplayStatics.GetActorOfClass` "/Game/Blueprints/BP_CheckpointManager.BP_CheckpointManager_C"))
  (set `self.CheckpointManager` _returnvalue)
  (bind _returnvalue_2 (`|CreateWidget` "/Game/Blueprints/UI/WBP_MainMenu.WBP_MainMenu_C" self))
  (`UserWidget.AddToViewport` _returnvalue_2 0)
  (bind _returnvalue_3 (`|CreateWidget` "/Game/Blueprints/UI/WBP_PlayerHUD.WBP_PlayerHUD_C" self))
  (bind _output_get (set `self.PlayerHUD` _returnvalue_3))
  (`UserWidget.AddToViewport` _output_get 0))

(event `self.RespawnBP`
  (bind _asbp_game_mode (cast `/Game/Blueprints/BP_GameMode` (`GameplayStatics.GetGameMode`)))
  (if (`/Game/Blueprints/BP_GameMode.IsHardcore` _asbp_game_mode)
    (`/Game/Blueprints/UI/WBP_PlayerHUD.ShowMessage` (`self.PlayerHUD`) "No checkpoints in hardcore." 2.0)
    (else
      (bind _returnvalue (`Blob_CheckpointManager.GetCheckpointLocation` (`self.CheckpointManager`)))
      (`self.K2_SetActorLocation` (`self.K2_GetPawn`) (+ _returnvalue (0.0 0.0 150.0)) false true)
      (`SceneComponent.K2_SetRelativeRotation` :`self` (`Blob_PlayerCharacter.CameraArm` (`self.PlayerCharacter`))))))

(event `self.OpenPauseMenu`
  (bind _returnvalue (`|CreateWidget` "/Game/Blueprints/UI/WBP_MainMenu.WBP_MainMenu_C" self))
  (`UserWidget.AddToViewport` _returnvalue 0)
  (`GameplayStatics.SetGlobalTimeDilation` 0.0)
  (`WidgetBlueprintLibrary.SetInputMode_UIOnlyEx` self _returnvalue)
  (set `self.bShowMouseCursor` true))

(event `self.OnCheckpointReachedBP`
  (params (Index :type Integer))
  (`/Game/Blueprints/UI/WBP_PlayerHUD.OnCheckpointReached` (`self.PlayerHUD`) Index))

(event `StartGame`
  (`/Game/Blueprints/UI/WBP_PlayerHUD.InitAndStart` :`self` (`self.PlayerHUD`)))

(fn `ShowMessage`
  (params (Message :type Text) (Time :type "Float (double-precision)"))
  (`/Game/Blueprints/UI/WBP_PlayerHUD.ShowMessage` (`self.PlayerHUD`) Message Time))

(fn `UserConstructionScript`)