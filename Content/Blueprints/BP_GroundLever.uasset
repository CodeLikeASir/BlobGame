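; BP_GroundLever is a ground lever that switches attached actors on and off.
; BeginPlay tilts the handle to its starting angle and caches a debug text widget.
; Tick derives IsOn from the sign of the handle's relative roll, firing toggle events only when the state changes.
; Those events forward the change to directly attached actors via Blob_Toggleable, so wiring is done by actor attachment.
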(event `self.ReceiveBeginPlay`
  (bind _aswbp_debug_text (cast `/Game/Blueprints/UI/WBP_DebugText` (`WidgetComponent.GetWidget` (`self.Widget`))))
  (set `self.WBP` _aswbp_debug_text)
  (`SceneComponent.K2_SetRelativeRotation` (`self.LeverHandle`) (struct :`Roll` -30.0) false false))

(event `self.ReceiveTick`
  (params (DeltaSeconds :type "Float (single-precision)"))
  (bind _relativerotation_roll (`KismetMathLibrary.BreakRotator` (`SceneComponent.RelativeRotation` (`self.LeverHandle`))))
  (bind _returnvalue (> _relativerotation_roll 0.0))
  (if (!= _returnvalue (`self.IsOn`))
    (bind _output_get (set `self.IsOn` _returnvalue))
    (if _output_get
      (`self.OnToggleOn`)
      (else
        (`self.OnToggleOff`)))))

(event `OnToggleOn`
  (for _array_element (`self.GetAttachedActors` true)
    (bind _asblob_toggleable (cast `Blob_Toggleable` _array_element))
    (`Blob_Toggleable.OnToggleOn` _asblob_toggleable)))

(event `OnToggleOff`
  (for _array_element (`self.GetAttachedActors` true)
    (bind _asblob_toggleable (cast `Blob_Toggleable` _array_element))
    (`Blob_Toggleable.OnToggleOff` _asblob_toggleable)))

(fn `UserConstructionScript`)