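; BP_GroundButton is a ground button that switches its attached Blob_Toggleable actors on and off.
; On BeginPlay it collects those actors from its directly attached children.
; Each Tick it compares GetZOffset against separate on and off thresholds, changing state only when the relevant one is crossed.
; Each change swaps the button material and calls OnToggleOn or OnToggleOff on every collected actor.
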(event `self.ReceiveBeginPlay`
  (for _array_element (`self.GetAttachedActors` true)
    (bind _asblob_toggleable (cast `Blob_Toggleable` _array_element))
    (`KismetArrayLibrary.Array_Add` (`self.Toggleables`) _asblob_toggleable)))

(event `self.ReceiveTick`
  (params (DeltaSeconds :type "Float (single-precision)"))
  (bind _offset (`self.GetZOffset`))
  (if (`self.IsOn`)
    (if (> _offset (`self.OffThreshold`))
      (set `self.IsOn` false)
      (`self.OnToggled` :!label _label))
    (elif (< _offset (`self.OnThreshold`))
      (set `self.IsOn` true)
      (goto _label))))

(event `OnToggled`
  (bind _button (`self.Button`))
  (if (`self.IsOn`)
    (`PrimitiveComponent.SetMaterial` _button 0 (`self.OnMaterial`))
    (else
      (`PrimitiveComponent.SetMaterial` _button 0 (`self.OffMaterial`))))
  (for _array_element (`self.Toggleables`)
    (if (`self.IsOn`)
      (`Blob_Toggleable.OnToggleOn` _array_element)
      (else
        (`Blob_Toggleable.OnToggleOff` _array_element)))))

(fn `UserConstructionScript`)