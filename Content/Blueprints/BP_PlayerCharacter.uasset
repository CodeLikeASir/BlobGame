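; Player character Blueprint for a blob with a charged jump, handling its visual feedback and debug display.
; Tick feeds ChargeProgress to a dynamic body material, shows the grounded state as green or red widget text, and publishes position and highest Z reached to a material parameter collection.
; Jump release plays a timeline easing the mesh from squished to base scale.
; Downforce events only print debug strings.
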(event `self.ReceiveBeginPlay`
  (bind _returnvalue (`PrimitiveComponent.CreateDynamicMaterialInstance` (`self.BlobMesh`) 0 "/Game/Meshes/Mat_Body.Mat_Body" "None"))
  (set `self.Material` _returnvalue)
  (`PrimitiveComponent.SetPhysMaterialOverride` (`self.CapsuleComponent`) "/Game/PM_Blob.PM_Blob")
  (bind _asbp_player_controller (cast `/Game/Blueprints/BP_PlayerController` (`GameplayStatics.GetPlayerController` 0)))
  (set `self.PC` _asbp_player_controller)
  (bind _aswbp_debug_text (cast `/Game/Blueprints/UI/WBP_DebugText` (`WidgetComponent.GetWidget` (`self.Widget`))))
  (set `self.DebugWBP` _aswbp_debug_text))

(event `self.ReceiveTick`
  (params (DeltaSeconds :type "Float (single-precision)"))
  (bind _bisgrounded (`self.bIsGrounded`))
  (`MaterialInstanceDynamic.SetScalarParameterValue` (`self.Material`) "ChargeProgress" (`self.ChargeProgress`))
  (`self.UpdatePlayerPos`)
  (`/Game/Blueprints/UI/WBP_DebugText.SetText` (`self.DebugWBP`) (`KismetTextLibrary.Conv_BoolToText` _bisgrounded) (`KismetMathLibrary.SelectColor` (struct :`G` 1.0 :`A` 1.0) (struct :`R` 1.0 :`A` 1.0) _bisgrounded)))

(event `self.ReleaseJumpBP`
  (bind (_direction _meshscalelerpalpha) (`Timeline|ResetScale` :!via `PlayFromStart`)
    (:`Update`
      (`SceneComponent.SetRelativeScale3D` (`self.BlobMesh`) (`KismetMathLibrary.VLerp` (`self.SquishScale`) (`self.BaseScale`) _meshscalelerpalpha)))))

(event `self.StartDownforceBP`
  (`KismetSystemLibrary.PrintString` "Heavy"))

(event `self.StopDownforceBP`
  (`KismetSystemLibrary.PrintString` "Light"))

(fn `UpdatePlayerPos`
  (bind _returnvalue (`self.K2_GetActorLocation`))
  (bind _z (.z _returnvalue))
  (`KismetMaterialLibrary.SetVectorParameterValue` (`self.ParamCollection`) "PlayerPosition" (`KismetMathLibrary.Conv_VectorToLinearColor` _returnvalue))
  (if (> _z (`self.HighestZ`))
    (bind _output_get (set `self.HighestZ` _z))
    (`KismetMaterialLibrary.SetScalarParameterValue` (`self.ParamCollection`) "HighestPlayerPosition" _output_get)
    (return)
    (else
      (return))))

(fn `UserConstructionScript`)